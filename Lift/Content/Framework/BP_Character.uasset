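; BP_Character is a player character with axis-driven movement and look that calls lifts to floors from input actions.
; Floor1 to Floor3 actions each look up the BP_Lift actor and call LiftRun with a fixed floor number.
; FloorNumber instead uses the lift reference cached on BeginPlay, converting the pressed key's display name into the floor number passed to LiftRun.
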(event EventBeginPlay
  (bind _returnvalue (Actor|GetActorOfClass "/Game/Blueprint/BP_Lift.BP_Lift_C"))
  (Variables|Default|SetLiftActor _returnvalue))

(event Input|ActionEvents|InputActionFloor1
  (params (Key :type Key%20Structure :default "None"))
  (:Pressed
    (bind _returnvalue (Actor|GetActorOfClass "/Game/Blueprint/BP_Lift.BP_Lift_C"))
    (Default|LiftRun _returnvalue 1.0)))

(event Input|ActionEvents|InputActionFloor2
  (params (Key :type Key%20Structure :default "None"))
  (:Pressed
    (bind _returnvalue (Actor|GetActorOfClass "/Game/Blueprint/BP_Lift.BP_Lift_C"))
    (Default|LiftRun _returnvalue 2.0)))

(event Input|ActionEvents|InputActionFloor3
  (params (Key :type Key%20Structure :default "None"))
  (:Pressed
    (bind _returnvalue (Actor|GetActorOfClass "/Game/Blueprint/BP_Lift.BP_Lift_C"))
    (Default|LiftRun _returnvalue 3.0)))

(event Input|ActionEvents|InputActionFloorNumber
  (params (Key :type Key%20Structure :default "None"))
  (:Pressed
    (Default|LiftRun (Variables|Default|GetLiftActor) (Math|Conversions|ToFloat(Integer) (Utilities|String|ToString(Text) (Class|KismetInputLibrary|KeyGetDisplayName Key true))))))

(event Input|AxisEvents|InputAxisMoveForward
  (params (AxisValue :type Float%20%28single-precision%29))
  ;[1 1 1] 注释
  (Pawn|Input|AddMovementInput (Transformation|GetActorForwardVector) AxisValue false))

(event Input|AxisEvents|InputAxisMoveRight
  (params (AxisValue :type Float%20%28single-precision%29))
  ;[1 1 1] 注释
  (Pawn|Input|AddMovementInput (Transformation|GetActorRightVector) AxisValue false))

(event Input|AxisEvents|InputAxisTurnRight
  (params (AxisValue :type Float%20%28single-precision%29))
  ;[1 1 1] 注释
  (Pawn|Input|AddControllerYawInput AxisValue))

(event Input|AxisEvents|InputAxisLookUp
  (params (AxisValue :type Float%20%28single-precision%29))
  ;[1 1 1] 注释
  (Pawn|Input|AddControllerPitchInput AxisValue))

(fn ConstructionScript)