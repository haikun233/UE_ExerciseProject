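; Elevator actor that carries the lift between numbered floors and animates its two sliding doors through timelines.
; LiftRun ignores requests for the current floor or during playing animations, plays the door animation, waits, then lerps lift height at fixed floor spacing.
; Play rate scales inversely with floors travelled, keeping trip speed consistent.
; At departure and arrival it passes the floor to every BP_LiftDoor in the level; two older movement chains remain unwired.
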(event Custom|LiftRun
  (params (FloorNumber :type Float%20%28double-precision%29))
  (if (not (== FloorNumber (Variables|Default|GetStartFloor)))
    (if (not (Audio|Components|Audio|IsPlaying (Variables|Default|GetDoorAnim)))
      (if (not (Audio|Components|Audio|IsPlaying (Variables|Default|GetLiftAnimation3)))
        (Variables|Default|SetEndFloor FloorNumber)
        (Components|Timeline|SetPlayRate (Variables|Default|GetLiftAnimation3) (/ 1.0 (Math|Float|Absolute(Float) (- (Variables|Default|GetEndFloor) (Variables|Default|GetStartFloor)))))
        (CallFunction|OpenDoorAnim)
        (bind _outactors (Actor|GetAllActorsOfClass "/Game/Blueprint/BP_LiftDoor.BP_LiftDoor_C")) ; 搜索场景中所有指定类型的对象文件
        (Default|OpenLiftDoorAnim _outactors (Variables|Default|GetStartFloor))
        (Utilities|FlowControl|Delay 2.0)
        (bind _alpha (Timeline|LiftAnimation3 PlayFromStart)
          (:Update
            (Transformation|SetRelativeLocation (Variables|Default|GetLift) (Math|Vector|MakeVector 0.0 0.0 (Math|Float|Lerp (* (- (Variables|Default|GetStartFloor) 1.0) 3e+02) (* (- (Variables|Default|GetEndFloor) 1.0) 3e+02) _alpha)) false false))
          (:Finished
            (Variables|Default|SetStartFloor (Variables|Default|GetEndFloor))
            (CallFunction|OpenDoorAnim)
            (bind _outactors_2 (Actor|GetAllActorsOfClass "/Game/Blueprint/BP_LiftDoor.BP_LiftDoor_C"))
            (Default|OpenLiftDoorAnim _outactors_2 (Variables|Default|GetStartFloor))))))))

(event Custom|OpenDoorAnim
  (bind _alpha (Timeline|DoorAnim PlayFromStart)
    (:Update
      (Transformation|SetRelativeLocation (Variables|Default|GetLeftDoor) (Math|Vector|MakeVector (Math|Float|Lerp -25.0 -75.0 _alpha) 52.5 9.5e+02) false false)
      (Transformation|SetRelativeLocation (Variables|Default|GetRightDoor) (Math|Vector|MakeVector (Math|Float|Lerp 25.0 75.0 _alpha) 52.5 9.5e+02) false false))))

(fn ConstructionScript)